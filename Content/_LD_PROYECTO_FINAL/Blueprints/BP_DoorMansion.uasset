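; BP_DoorMansion is a mansion door actor that the player can interact with and open.
; Its trigger flags BP_Player as able to interact, passes the door's Id and shows a HUD prompt reflecting key possession, undoing this on exit.
; OpenDoor plays a timeline that moves the mesh along Z, then removes the Id index from the game mode's Doors array and destroys the actor.
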(event OnComponentBeginOverlap(DoorTrigger)
  (params (OverlappedComponent :type Primitive%20Component%20Object%20Reference) (OtherActor :type Actor%20Object%20Reference) (OtherComp :type Primitive%20Component%20Object%20Reference) (OtherBodyIndex :type Integer) (bFromSweep :type Boolean) (SweepResult :type Hit%20Result%20Structure%20%28by%20ref%29))
  (bind _asbp_player (Utilities|Casting|CastToBP_Player OtherActor))
  (Variables|/Game/_LD_PROYECTO_FINAL/Blueprints/BP_Player.BP_Player_C|SetcanInteractWithDoors _asbp_player true)
  (Variables|/Game/_LD_PROYECTO_FINAL/Blueprints/BP_Player.BP_Player_C|SetcurrentDoor _asbp_player (Variables|Default|Getid))
  (Default|ShowDoorTxt (Variables|/Game/_LD_PROYECTO_FINAL/Blueprints/GM_LDGameMode.GM_LDGameMode_C|Gethud (Variables|Default|GetgameManager)) (Variables|/Game/_LD_PROYECTO_FINAL/Blueprints/BP_Player.BP_Player_C|GethasKey _asbp_player)))

(event OnComponentEndOverlap(DoorTrigger)
  (params (OverlappedComponent :type Primitive%20Component%20Object%20Reference) (OtherActor :type Actor%20Object%20Reference) (OtherComp :type Primitive%20Component%20Object%20Reference) (OtherBodyIndex :type Integer))
  (bind _asbp_player (Utilities|Casting|CastToBP_Player OtherActor))
  (Variables|/Game/_LD_PROYECTO_FINAL/Blueprints/BP_Player.BP_Player_C|SetcanInteractWithDoors _asbp_player false)
  (Variables|/Game/_LD_PROYECTO_FINAL/Blueprints/BP_Player.BP_Player_C|SetcurrentDoor _asbp_player -10)
  (Default|HideDoorTxt (Variables|/Game/_LD_PROYECTO_FINAL/Blueprints/GM_LDGameMode.GM_LDGameMode_C|Gethud (Variables|Default|GetgameManager))))

(event Custom|OpenDoor
  (bind _doormesh (Variables|Default|GetDoorMesh))
  (bind _returnvalue (Transformation|GetWorldLocation _doormesh))
  (bind _posz (Timeline|OpeningAnim PlayFromStart)
    (:Update
      (Transformation|SetWorldLocation _doormesh (Math|Vector|MakeVector (.x _returnvalue) (.y _returnvalue) _posz) false false))
    (:Finished
      (Utilities|Array|RemoveIndex (Variables|/Game/_LD_PROYECTO_FINAL/Blueprints/GM_LDGameMode.GM_LDGameMode_C|Getdoors (Variables|Default|GetgameManager)) (Variables|Default|Getid))
      (Actor|DestroyActor))))

(event EventBeginPlay
  (bind _asgm_ldgame_mode (Utilities|Casting|CastToGM_LDGameMode (Game|GetGameMode)))
  (Variables|Default|SetgameManager _asgm_ldgame_mode))

(fn ConstructionScript)
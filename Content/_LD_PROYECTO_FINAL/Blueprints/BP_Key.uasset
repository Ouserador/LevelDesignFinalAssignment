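; BP_Key is a rotating pickup that, on player overlap, sets the player's HasKey flag and shows key text on the HUD.
; A timeline spins it on yaw, while the overlap removes its Id index from the game mode's Keys array and decrements NumKeys.
; When no keys remain, it destroys doors flagged IsFinalDoor; the key destroys itself after that or when keys remain.
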(event OnComponentBeginOverlap(KeyTrigger)
  (params (OverlappedComponent :type Primitive%20Component%20Object%20Reference) (OtherActor :type Actor%20Object%20Reference) (OtherComp :type Primitive%20Component%20Object%20Reference) (OtherBodyIndex :type Integer) (bFromSweep :type Boolean) (SweepResult :type Hit%20Result%20Structure%20%28by%20ref%29))
  (bind _gamemanager (Variables|Default|GetgameManager))
  (bind _gamemanager_2 (Variables|Default|GetgameManager))
  (bind _numkeys (Variables|/Game/_LD_PROYECTO_FINAL/Blueprints/GM_LDGameMode.GM_LDGameMode_C|GetnumKeys _gamemanager))
  (bind _asbp_player (Utilities|Casting|CastToBP_Player OtherActor))
  (Variables|/Game/_LD_PROYECTO_FINAL/Blueprints/BP_Player.BP_Player_C|SethasKey _asbp_player true)
  (Default|AddKeyTxt (Variables|/Game/_LD_PROYECTO_FINAL/Blueprints/GM_LDGameMode.GM_LDGameMode_C|Gethud _gamemanager_2))
  (Utilities|Array|RemoveIndex (Variables|/Game/_LD_PROYECTO_FINAL/Blueprints/GM_LDGameMode.GM_LDGameMode_C|Getkeys _gamemanager_2) (Variables|Default|Getid))
  (Math|Integer|DecrementInt (Variables|/Game/_LD_PROYECTO_FINAL/Blueprints/GM_LDGameMode.GM_LDGameMode_C|GetnumKeys (Variables|Default|GetgameManager))
    (:%20%20
      (if (<= _numkeys 0)
        (for _array_element (Variables|/Game/_LD_PROYECTO_FINAL/Blueprints/GM_LDGameMode.GM_LDGameMode_C|Getdoors (Variables|Default|GetgameManager))
          (if (Variables|/Game/_LD_PROYECTO_FINAL/Blueprints/BP_Door.BP_Door_C|GetisFinalDoor _array_element)
            (Actor|DestroyActor _array_element)
            (Development|PrintString "Hello")
            (Actor|DestroyActor)
            (Development|PrintString (Utilities|String|ToString(Integer) _numkeys))))
        (else
          (Actor|DestroyActor)
          (Development|PrintString (Utilities|String|ToString(Integer) _numkeys)))))))

(event EventBeginPlay
  (bind _defaultsceneroot (Variables|Default|GetDefaultSceneRoot))
  (bind _returnvalue (Transformation|GetWorldRotation _defaultsceneroot))
  (Utilities|FlowControl|Sequence
    (:then_0
      (bind _asgm_ldgame_mode (Utilities|Casting|CastToGM_LDGameMode (Game|GetGameMode)))
      (Variables|Default|SetgameManager _asgm_ldgame_mode))
    (:then_1
      (bind _rotz (Timeline|Rotation Play)
        (:Update
          (Transformation|SetWorldRotation _defaultsceneroot (Math|Rotator|MakeRotator (.roll _returnvalue) (.pitch _returnvalue) _rotz) false false))))))

(fn ConstructionScript)
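; BP_Trol is an enemy troll that wanders the level, chases the player on sight and ends their run on contact.
; It roams by repeatedly moving to random reachable points within a radius of itself.
; PawnSensing redirects it to the seen player's current location, and a failed chase move resumes roaming after a short delay.
; Player overlap with its DeathZone calls PlayerCaughtOrDead on the GM_LDGameMode cached at BeginPlay.
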(event OnSeePawn(PawnSensing)
  (params (Pawn :type Pawn%20Object%20Reference))
  (bind _asbp_player (Utilities|Casting|CastToBP_Player Pawn))
  (AI|AIMoveTo self (Transformation|GetActorLocation _asbp_player) 0 5e+01 false
    (:OnFail
      (Utilities|FlowControl|RetriggerableDelay 0.5)
      (CallFunction|Roaming))))

(event OnComponentBeginOverlap(DeathZone)
  (params (OverlappedComponent :type Primitive%20Component%20Object%20Reference) (OtherActor :type Actor%20Object%20Reference) (OtherComp :type Primitive%20Component%20Object%20Reference) (OtherBodyIndex :type Integer) (bFromSweep :type Boolean) (SweepResult :type Hit%20Result%20Structure%20%28by%20ref%29))
  (Utilities|Casting|CastToBP_Player OtherActor)
  (Default|PlayerCaughtorDead (Variables|Default|GetgameManager)))

(event Custom|Roaming
  (AI|AIMoveTo self (.RandomLocation (AI|Navigation|GetRandomReachablePointinRadius (Transformation|GetActorLocation) 2e+03 0 0)) 0 5.0 false
    (:OnSuccess
      (Utilities|FlowControl|RetriggerableDelay 0.5)
      (CallFunction|Roaming))))

(event EventBeginPlay
  (bind _asgm_ldgame_mode (Utilities|Casting|CastToGM_LDGameMode (Game|GetGameMode)))
  (Variables|Default|SetgameManager _asgm_ldgame_mode)
  (CallFunction|Roaming))

(fn ConstructionScript)
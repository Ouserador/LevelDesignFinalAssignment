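; Game mode for a level that gathers the player, doors, keys and spikes and creates the HUD.
; On BeginPlay it caches those actors, sets each door, key and spike Id to its array index, and adds WB_HUD to the viewport.
; It then switches input to game-only and hides the mouse cursor.
; The PlayerCaughtOrDead and PlayerWon events are empty stubs.
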(event Custom|PlayerCaughtOrDead)

(event Custom|PlayerWon)

(event EventBeginPlay
  (bind _returnvalue (Game|GetPlayerController 0))
  (Utilities|FlowControl|Sequence
    (:then_0
      (CallFunction|GetEntitiesinGame))
    (:then_1
      (Input|SetInputModeGameOnly _returnvalue false)
      (Variables|/Script/Engine.PlayerController|SetbShowMouseCursor _returnvalue false))))

(fn ConstructionScript)

(fn GetEntitiesinGame
  (Utilities|FlowControl|Sequence
    (:then_0
      (bind _returnvalue (Actor|GetActorOfClass "/Game/_LD_PROYECTO_FINAL/Blueprints/BP_Player.BP_Player_C"))
      (Variables|Default|Setplayer _returnvalue))
    (:then_1
      (bind _outactors (Actor|GetAllActorsOfClass "/Game/_LD_PROYECTO_FINAL/Blueprints/BP_Door.BP_Door_C"))
      (bind _output_get (Variables|Default|Setdoors _outactors))
      (for (_array_element _array_index) _output_get
        (Variables|/Game/_LD_PROYECTO_FINAL/Blueprints/BP_Door.BP_Door_C|Setid _array_element _array_index)))
    (:then_2
      (bind _outactors_2 (Actor|GetAllActorsOfClass "/Game/_LD_PROYECTO_FINAL/Blueprints/BP_Key.BP_Key_C"))
      (bind _output_get_2 (Variables|Default|Setkeys _outactors_2))
      (for (_array_element_2 _array_index_2) _output_get_2
        (Variables|/Game/_LD_PROYECTO_FINAL/Blueprints/BP_Key.BP_Key_C|Setid _array_element_2 _array_index_2)))
    (:then_3
      (bind _outactors_3 (Actor|GetAllActorsOfClass "/Game/_LD_PROYECTO_FINAL/Blueprints/BP_Spikes.BP_Spikes_C"))
      (bind _output_get_3 (Variables|Default|Setspikes _outactors_3))
      (for (_array_element_3 _array_index_3) _output_get_3
        (Variables|/Game/_LD_PROYECTO_FINAL/Blueprints/BP_Spikes.BP_Spikes_C|Setid _array_element_3 _array_index_3)))
    (:then_4
      (bind _returnvalue_2 (UserInterface|CreateWidget "/Game/_LD_PROYECTO_FINAL/UI/WB_HUD.WB_HUD_C"))
      (bind _output_get_4 (Variables|Default|Sethud _returnvalue_2))
      (UserInterface|Viewport|AddtoViewport _output_get_4 0))))